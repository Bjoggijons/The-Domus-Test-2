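; Bookshelf book actor that acts as a pullable switch, with a correct book triggering a door-opening puzzle response.
; BeginPlay stores the book's relative location and applies its configurable mesh.
; Clicks call Interact, while Interact_Book runs a timeline that lerps the book along local Y by a scaled PullDistance.
; When the timeline finishes on the correct book, it notifies the bookshelf reference and plays a door-opened sound.
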(event OnClicked(Book)
  (params (TouchedComponent :type Primitive%20Component%20Object%20Reference) (ButtonPressed :type Key%20Structure :default "None"))
  (CallFunction|Interact))

(event Custom|Interact_Book
  (bind _originallocation (Variables|Default|GetOriginalLocation))
  (bind _alpha (Timeline|Interact_Timeline Play)
    (:Update
      (Transformation|SetRelativeLocation (Variables|Default|GetBook) (Math|Vector|Lerp(Vector) _originallocation (+ _originallocation (* "0.000000,0.200000,0.000000" (Variables|Default|GetPullDistance))) _alpha) false false))
    (:Finished
      (if (Variables|Default|GetIsCorrectBook)
        (Default|OnCorrectBookPulled (Variables|Default|GetBookshelfRef))
        (Development|PrintString "door opening")
        (Audio|PlaySound2D "/Game/ReactionQuest/Audio/Ambient/SFX_DoorOpened.SFX_DoorOpened" 1.0 1.0 0.0 0 0)))))

(event Custom|InteractFlipFlop
  (Utilities|FlowControl|FlipFlop
    (:A
      (CallFunction|InteractBook))))

(event EventBeginPlay
  (Variables|Default|SetOriginalLocation (Variables|/Script/Engine.SceneComponent|GetRelativeLocation (Variables|Default|GetBook)))
  (Components|StaticMesh|SetStaticMesh (Variables|Default|GetBook) (Variables|Default|GetBooks)))

(fn ConstructionScript)