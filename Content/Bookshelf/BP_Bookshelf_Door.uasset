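; Bookshelf door Blueprint that swings its Door component open when the OpenDoor event is called.
; BeginPlay caches the door's relative rotation, and a timeline's Alpha lerps from it toward the open rotation.
; The open target adds 180° of yaw, then combines that with the original rotation again, so any nonzero starting rotation is applied twice.
; No close or reverse path exists.
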(event Custom|OpenDoor
  (bind _originalrotation (Variables|Default|GetOriginalRotation))
  (bind (_roll _pitch _yaw) (Math|Rotator|BreakRotator _originalrotation))
  (bind _alpha (Timeline|DoorOpenTimeline Play)
    (:Update
      (Transformation|SetRelativeRotation (Variables|Default|GetDoor) (Math|Rotator|Lerp(Rotator) _originalrotation (Math|Rotator|CombineRotators (Math|Rotator|MakeRotator _roll _pitch (+ _yaw 1.8e+02)) _originalrotation) _alpha) false false))))

(event EventBeginPlay
  (Variables|Default|SetOriginalRotation (Variables|/Script/Engine.SceneComponent|GetRelativeRotation (Variables|Default|GetDoor))))

(fn ConstructionScript)