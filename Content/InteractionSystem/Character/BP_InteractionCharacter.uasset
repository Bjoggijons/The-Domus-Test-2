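; Networked first-person player character with movement, sprint, aim zoom, idle/walk camera shakes and interaction with doors, buttons and loot.
; Tick bounces through Server then Client RPCs to run camera shake and a camera line trace.
; The trace toggles focus on tagged actors and sends the focused actor to the server.
; Interact input multicasts via the server, messaging that actor if its tag matches; sprint speed is also multicast.
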(event Custom|On%20Aiming
  (params (Aim :type Boolean))
  ;[1 0.8509 0.3646 0.5] Character Action
  ;;[1 1 1 0.5] Aim (input)
  (if Aim
    (bind _alpha (Timeline|Timeline%20Aim Play)
      (:Update
        (Camera|SetFieldOfView (Variables|Default|GetCamera) (Math|Float|Lerp 1.1e+02 9e+01 _alpha))))
    (else
      (Timeline|Timeline%20Aim Reverse))))

(event Custom|Line%20Trace%20Player%20%28client%29
  ;[0.4901 1 0.6446 0.5] Event
  ;;[1 1 1 0.5] Line Trace (client)
  (CallFunction|LineTracePlayer))

(event Custom|Line%20Trace%20Player%20%28server%29
  ;[0.4901 1 0.6446 0.5] Event
  ;;[1 1 1 0.5] Line Trace (client)
  (CallFunction|LineTracePlayer(client)))

(event Custom|Set%20Max%20Walk%20Speed%20%28Server%29
  (params (Max%20Walk%20Speed :type Float%20%28single-precision%29))
  ;[0.4901 1 0.6446 0.5] Event
  ;;[1 1 1 0.5] Max Walk Speed (server)
  (CallFunction|MaxWalkSpeed(multicast) Max%20Walk%20Speed))

(event Custom|Max%20Walk%20Speed%20%28multicast%29
  (params (Max%20Walk%20Speed :type Float%20%28single-precision%29))
  ;[0.4901 1 0.6446 0.5] Event
  ;;[1 1 1 0.5] Max Walk Speed (server)
  (Variables|/Script/Engine.CharacterMovementComponent|SetMaxWalkSpeed (Variables|Character|GetCharacterMovement) Max%20Walk%20Speed))

(event Custom|Camera%20Shake%20%28server%29
  ;[0.4901 1 0.6446 0.5] Event
  ;;[1 1 1 0.5] Camera Shake (Client)
  (CallFunction|CameraShake(client)))

(event Custom|Camera%20Shake%20%28client%29
  ;[0.4901 1 0.6446 0.5] Event
  ;;[1 1 1 0.5] Camera Shake (Client)
  (CallFunction|CameraShake))

(event Custom|Set%20Current%20Focused%20Actor%20%28server%29
  (params (CurrentFocusedActor :type Actor%20Object%20Reference))
  ;[0.4901 1 0.6446 0.5] Event
  ;;[1 1 1 0.5] Set Current Focused Actor (server)
  (Variables|Default|SetCurrentFocusedActor CurrentFocusedActor))

(event Custom|Try%20To%20Interact%20%28server%29
  ;[0.4901 1 0.6446 0.5] Event
  ;;[1 1 1 0.5] Interaction (server)
  (CallFunction|TrytoInteract(multicast)))

(event Custom|Try%20To%20Interact%20%28multicast%29
  ;[0.4901 1 0.6446 0.5] Event
  ;;[1 1 1 0.5] Interaction (server)
  (CallFunction|TrytoInteract))

(event Input|EnhancedActionEvents|EnhancedInputActionIA_Look
  (params (ActionValue :type Vector%202D%20Structure) (ElapsedSeconds :type Float%20%28double-precision%29) (TriggeredSeconds :type Float%20%28double-precision%29) (InputAction :type Input%20Action%20Object%20Reference :default "/Game/InteractionSystem/Character/Inputs/Actions/IA_Look.IA_Look"))
  ;[0.531 0.9223 1 0.5] Character Movement
  ;;[1 1 1 0.5] Look (input)
  (Pawn|Input|AddControllerYawInput (* (.x ActionValue) 0.32))
  (Pawn|Input|AddControllerPitchInput (* (.y ActionValue) 0.32)))

(event Input|EnhancedActionEvents|EnhancedInputActionIA_Move
  (params (ActionValue :type Vector%202D%20Structure) (ElapsedSeconds :type Float%20%28double-precision%29) (TriggeredSeconds :type Float%20%28double-precision%29) (InputAction :type Input%20Action%20Object%20Reference :default "/Game/InteractionSystem/Character/Inputs/Actions/IA_Move.IA_Move"))
  ;[0.531 0.9223 1 0.5] Character Movement
  ;;[1 1 1 0.5] Move (input)
  (Pawn|Input|AddMovementInput (Transformation|GetActorRightVector) (.x ActionValue) false)
  (Pawn|Input|AddMovementInput (Transformation|GetActorForwardVector) (.y ActionValue) false))

(event Input|EnhancedActionEvents|EnhancedInputActionIA_Sprint
  (params (ActionValue :type Boolean) (ElapsedSeconds :type Float%20%28double-precision%29) (TriggeredSeconds :type Float%20%28double-precision%29) (InputAction :type Input%20Action%20Object%20Reference :default "/Game/InteractionSystem/Character/Inputs/Actions/IA_Sprint.IA_Sprint"))
  ;[0.531 0.9223 1 0.5] Character Movement
  ;;[1 1 1 0.5] Sprint (input)
  (:Started
    (CallFunction|SetMaxWalkSpeed(Server) 3.2e+02))
  (:Completed
    (CallFunction|SetMaxWalkSpeed(Server) 2.4e+02)))

(event Input|EnhancedActionEvents|EnhancedInputActionIA_Jump
  (params (ActionValue :type Boolean) (ElapsedSeconds :type Float%20%28double-precision%29) (TriggeredSeconds :type Float%20%28double-precision%29) (InputAction :type Input%20Action%20Object%20Reference :default "/Game/InteractionSystem/Character/Inputs/Actions/IA_Jump.IA_Jump"))
  ;[0.531 0.9223 1 0.5] Character Movement
  ;;[1 1 1 0.5] Jump (input)
  (:Started
    (Character|Jump)))

(event Input|EnhancedActionEvents|EnhancedInputActionIA_Aim
  (params (ActionValue :type Boolean) (ElapsedSeconds :type Float%20%28double-precision%29) (TriggeredSeconds :type Float%20%28double-precision%29) (InputAction :type Input%20Action%20Object%20Reference :default "/Game/InteractionSystem/Character/Inputs/Actions/IA_Aim.IA_Aim"))
  ;[1 0.8509 0.3646 0.5] Character Action
  ;;[1 1 1 0.5] Aim (input)
  (:Started
    (CallFunction|OnAiming true))
  (:Completed
    (CallFunction|OnAiming false)))

(event Input|EnhancedActionEvents|EnhancedInputActionIA_Interact
  (params (ActionValue :type Boolean) (ElapsedSeconds :type Float%20%28double-precision%29) (TriggeredSeconds :type Float%20%28double-precision%29) (InputAction :type Input%20Action%20Object%20Reference :default "/Game/InteractionSystem/Character/Inputs/Actions/IA_Interact.IA_Interact"))
  ;[1 0.8509 0.3646 0.5] Character Action
  ;;[1 1 1 0.5] IA_Interact
  (:Started
    (CallFunction|TrytoInteract(server))))

(event EventBeginPlay
  ;[1 1 1 0.5] Begin play
  (Class|PrimitiveComponent|SetOwnerNoSee (Variables|Character|GetMesh) true))

(event EventTick
  (params (DeltaSeconds :type Float%20%28single-precision%29))
  ;[0 1 0.00255 0.5] Tick
  (CallFunction|CameraShake(server))
  (CallFunction|LineTracePlayer(server)))

(fn ConstructionScript)

(fn CameraShake
  (bind _returnvalue (Transformation|GetVelocity))
  (bind _returnvalue_2 (Math|Vector|VectorLength _returnvalue))
  (if (and (> _returnvalue_2 0.0) (Character|CanJump))
    (if (< _returnvalue_2 3.2e+02)
      ;[1 1 1 0.5] Walk
      (Game|Feedback|ClientStartCameraShake (Game|GetPlayerController 0) "/Game/InteractionSystem/Character/Camera/LCS_CameraWalk.LCS_CameraWalk_C" 1.0 "CameraLocal" "0, 0, 0"))
    (else
      ;[1 1 1 0.5] Idle
      (Game|Feedback|ClientStartCameraShake (Game|GetPlayerController 0) "/Game/InteractionSystem/Character/Camera/LCS_CameraIdle.LCS_CameraIdle_C" 1.0 "CameraLocal" "0, 0, 0"))))

(fn LineTracePlayer
  (bind _returnvalue (Game|GetPlayerCameraManager 0))
  (bind _returnvalue_2 (Transformation|GetActorLocation _returnvalue))
  (bind (_outhit _returnvalue_3) (Collision|LineTraceByChannel _returnvalue_2 (+ _returnvalue_2 (* (Math|Vector|GetForwardVector (Transformation|GetActorRotation _returnvalue)) (Variables|Default|GetMaxDistance))) "TraceTypeQuery1" false 0 "None"))
  (if (and _returnvalue_3 (Utilities|IsValid (.HitActor (Collision|BreakHitResult _outhit))))
    (bind _output_get (LocalVariables|SetLocal%20HitActor (.HitActor (Collision|BreakHitResult _outhit))))
    (if (> (Utilities|Array|Length (Variables|/Script/Engine.Actor|GetTags _output_get)) 0)
      (bind _currentfocusedactor (Variables|Default|GetCurrentFocusedActor)
        (:then
          (Class|BPIInteraction|FocusInteraction(Message) _currentfocusedactor false))
        (:else
          _))
      (Class|BPIInteraction|FocusInteraction(Message) (LocalVariables|GetLocal%20HitActor) true)
      (CallFunction|SetCurrentFocusedActor(server) (LocalVariables|GetLocal%20HitActor))
      (else
        (bind _currentfocusedactor_2 (Variables|Default|GetCurrentFocusedActor :!label _label)
          (:then
            (Class|BPIInteraction|FocusInteraction(Message) _currentfocusedactor_2 false))
          (:else
            _))
        (bind _output_get_2 (LocalVariables|SetLocal%20HitActor 0))
        (CallFunction|SetCurrentFocusedActor(server) _output_get_2)))
    (else
      (goto _label))))

(fn TrytoInteract
  (Utilities|IsValid (Variables|Default|GetCurrentFocusedActor)
    (:Is%20Valid
      ;[1 1 1 0.5] Door?
      (if (Actor|ActorHasTag (Variables|Default|GetCurrentFocusedActor) "Door")
        (Class|BPIInteraction|InteractwithActor(Message) (Variables|Default|GetCurrentFocusedActor) :!label _label)
        (else
          ;[1 1 1 0.5] Light Button?
          (if (Actor|ActorHasTag (Variables|Default|GetCurrentFocusedActor) "LightButton")
            (goto _label)
            (else
              ;[1 1 1 0.5] Door Button?
              (if (Actor|ActorHasTag (Variables|Default|GetCurrentFocusedActor) "DoorButton")
                (goto _label)
                (else
                  ;[1 1 1 0.5] Loot?
                  (if (Actor|ActorHasTag (Variables|Default|GetCurrentFocusedActor) "Loot")
                    (goto _label)))))))))))