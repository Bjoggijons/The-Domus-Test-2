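; BP_DoorWithOverlap is a door that swings open when a BP_InteractionCharacter enters its BoxForward volume and closes when that character leaves.
; Begin and end overlap call a server event with a reverse flag, which relays it through a multicast.
; Each machine then plays or reverses TimelineDoor, whose alpha drives the door's relative yaw between closed and open.
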(event OnComponentBeginOverlap(BoxForward)
  (params (OverlappedComponent :type Primitive%20Component%20Object%20Reference) (OtherActor :type Actor%20Object%20Reference) (OtherComp :type Primitive%20Component%20Object%20Reference) (OtherBodyIndex :type Integer) (bFromSweep :type Boolean) (SweepResult :type Hit%20Result%20Structure%20%28by%20ref%29))
  ;[1 1 1 0.5] Overlap Event
  (Utilities|Casting|CastToBP_InteractionCharacter OtherActor)
  (CallFunction|OpenDoor(server) false))

(event OnComponentEndOverlap(BoxForward)
  (params (OverlappedComponent :type Primitive%20Component%20Object%20Reference) (OtherActor :type Actor%20Object%20Reference) (OtherComp :type Primitive%20Component%20Object%20Reference) (OtherBodyIndex :type Integer))
  ;[1 1 1 0.5] Overlap Event
  (Utilities|Casting|CastToBP_InteractionCharacter OtherActor)
  (CallFunction|OpenDoor(server) true))

(event Custom|Open%20Door%20%28server%29
  (params (Reverse? :type Boolean))
  ;[1 1 1 0.5] Open Door (server)
  (CallFunction|OpenDoor(Multicast) Reverse?))

(event Custom|Open%20Door%20%28Multicast%29
  (params (Reverse? :type Boolean))
  (bind _timeline_door (Variables|Default|GetTimeline%20Door))
  ;[1 1 1 0.5] Open Door (multicast)
  (if Reverse?
    (Utilities|String|Reverse _timeline_door)
    (else
      (Audio|Components|Audio|Play _timeline_door))))

(fn ConstructionScript)