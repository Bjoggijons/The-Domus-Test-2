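; BP_DoorWithInteraction is an interactable door that toggles open and closed through interface events.
; Interacting flips DoorIsOpen and passes it to a multicast, which plays or reverses a timeline meant to swing the door's yaw.
; Focus events set a custom depth stencil on the door and notify its WBP_NearestInteraction widget.
; A sphere overlap shows the widget for the local player character and clears it and the highlight on exit.
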(event OnComponentBeginOverlap(Sphere)
  (params (OverlappedComponent :type Primitive%20Component%20Object%20Reference) (OtherActor :type Actor%20Object%20Reference) (OtherComp :type Primitive%20Component%20Object%20Reference) (OtherBodyIndex :type Integer) (bFromSweep :type Boolean) (SweepResult :type Hit%20Result%20Structure%20%28by%20ref%29))
  ;[0.6445 0.8228 1 0.502] Local Overlap Event
  (if (== (Game|GetPlayerCharacter 0) OtherActor)
    (Utilities|Casting|CastToBP_InteractionCharacter OtherActor)
    (Development|SetHiddeninGame (Variables|Default|GetWidget) false false)))

(event OnComponentEndOverlap(Sphere)
  (params (OverlappedComponent :type Primitive%20Component%20Object%20Reference) (OtherActor :type Actor%20Object%20Reference) (OtherComp :type Primitive%20Component%20Object%20Reference) (OtherBodyIndex :type Integer))
  (bind _door (Variables|Default|GetDoor))
  (bind _widget (Variables|Default|GetWidget))
  ;[0.6445 0.8228 1 0.502] Local Overlap Event
  (if (== OtherActor (Game|GetPlayerCharacter 0))
    (Utilities|Casting|CastToBP_InteractionCharacter OtherActor)
    (Rendering|SetRenderCustomDepth _door false)
    (Rendering|SetCustomDepthStencilValue _door 0)
    (if (Rendering|IsVisible _widget)
      (Development|SetHiddeninGame _widget true false))))

(event Custom|Open%20Door%20%28multicast%29
  (params (DoorIsOpen? :type Boolean))
  (bind _timeline_door (Variables|Default|GetTimeline%20Door))
  ;[1 1 1 0.5] Open Door (multicast)
  (if DoorIsOpen?
    (Audio|Components|Audio|Play _timeline_door)
    (else
      (Utilities|String|Reverse _timeline_door))))

(event EventBeginPlay
  ;[1 1 1 0.5] Begin Play
  (bind _aswbp_nearest_interaction (Utilities|Casting|CastToWBP_NearestInteraction (UserInterface|GetWidget (Variables|Default|GetWidget))))
  (Variables|Default|SetAs%20WBP%20Nearest%20Interaction _aswbp_nearest_interaction))

(event EventFocusInteraction
  (params (Focused :type Boolean))
  (bind _door (Variables|Default|GetDoor))
  (bind _door_2 (Variables|Default|GetDoor))
  (bind _widget (Variables|Default|GetWidget))
  (bind _widget_2 (Variables|Default|GetWidget))
  ;[1 1 1 0.5] Focus Interaction (interface)
  (if Focused
    ;[0.6445 0.8228 1 0.502] Local Visual
    (Rendering|SetRenderCustomDepth _door true)
    (Rendering|SetCustomDepthStencilValue _door 2)
    (if (Rendering|IsVisible _widget_2)
      _
      (else
        (Development|SetHiddeninGame _widget_2 false false)))
    (Default|OnFocused (Variables|Default|GetAs%20WBP%20Nearest%20Interaction) true)
    (else
      (Rendering|SetRenderCustomDepth _door_2 false)
      (Rendering|SetCustomDepthStencilValue _door_2 0)
      (if (Rendering|IsVisible _widget)
        _
        (else
          (Development|SetHiddeninGame _widget true false)))
      (Default|OnFocused (Variables|Default|GetAs%20WBP%20Nearest%20Interaction) false))))

(event EventInteractwithActor
  ;[1 1 1 0.5] Interact With Actor (interface)
  (if (Variables|Default|GetDoorIsOpen?)
    (Variables|Default|SetDoorIsOpen? false)
    (else
      (Variables|Default|SetDoorIsOpen? true)))
  (CallFunction|OpenDoor(multicast) (Variables|Default|GetDoorIsOpen?)))

(fn ConstructionScript)