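; BP_Loot is an interactable loot container whose lid opens once when the player interacts with it.
; An overlap sphere shows or hides a nearest-interaction widget for the local player character, and focus toggles the lid's custom-depth stencil highlight and notifies that widget.
; Interaction sets an open flag and calls a multicast event that plays a timeline to slide and tilt the lid.
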(event OnComponentBeginOverlap(Sphere)
  (params (OverlappedComponent :type Primitive%20Component%20Object%20Reference) (OtherActor :type Actor%20Object%20Reference) (OtherComp :type Primitive%20Component%20Object%20Reference) (OtherBodyIndex :type Integer) (bFromSweep :type Boolean) (SweepResult :type Hit%20Result%20Structure%20%28by%20ref%29))
  (if (== (Game|GetPlayerCharacter 0) OtherActor)
    (Utilities|Casting|CastToBP_InteractionCharacter OtherActor)
    (Development|SetHiddeninGame (Variables|Default|GetWidget) false false)))

(event OnComponentEndOverlap(Sphere)
  (params (OverlappedComponent :type Primitive%20Component%20Object%20Reference) (OtherActor :type Actor%20Object%20Reference) (OtherComp :type Primitive%20Component%20Object%20Reference) (OtherBodyIndex :type Integer))
  (bind _lid (Variables|Default|GetLid))
  (bind _widget (Variables|Default|GetWidget))
  (if (== OtherActor (Game|GetPlayerCharacter 0))
    (Utilities|Casting|CastToBP_InteractionCharacter OtherActor)
    (Rendering|SetRenderCustomDepth _lid false)
    (Rendering|SetCustomDepthStencilValue _lid 0)
    (if (Rendering|IsVisible _widget)
      (Development|SetHiddeninGame _widget true false))))

(event Custom|Open%20Lid%20%28multicast%29
  (Audio|Components|Audio|Play (Variables|Default|GetTimeline%20Lid)))

(event EventBeginPlay
  (bind _aswbp_nearest_interaction (Utilities|Casting|CastToWBP_NearestInteraction (UserInterface|GetWidget (Variables|Default|GetWidget))))
  (Variables|Default|SetAs%20WBP%20Nearest%20Interaction _aswbp_nearest_interaction))

(event EventInteractwithActor
  (if (not (Variables|Default|GetLidIsOpen?))
    (Variables|Default|SetLidIsOpen? true)
    (CallFunction|OpenLid(multicast))))

(event EventFocusInteraction
  (params (Focused :type Boolean))
  (bind _lid (Variables|Default|GetLid))
  (bind _lid_2 (Variables|Default|GetLid))
  (bind _widget (Variables|Default|GetWidget))
  (bind _widget_2 (Variables|Default|GetWidget))
  (if Focused
    (Rendering|SetRenderCustomDepth _lid true)
    (Rendering|SetCustomDepthStencilValue _lid 2)
    (if (Rendering|IsVisible _widget_2)
      _
      (else
        (Development|SetHiddeninGame _widget_2 false false)))
    (Default|OnFocused (Variables|Default|GetAs%20WBP%20Nearest%20Interaction) true)
    (else
      (Rendering|SetRenderCustomDepth _lid_2 false)
      (Rendering|SetCustomDepthStencilValue _lid_2 0)
      (if (Rendering|IsVisible _widget)
        _
        (else
          (Development|SetHiddeninGame _widget true false)))
      (Default|OnFocused (Variables|Default|GetAs%20WBP%20Nearest%20Interaction) false))))

(fn ConstructionScript)