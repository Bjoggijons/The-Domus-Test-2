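; BP_LightButton is an interactable push button that toggles a linked spotlight on and off.
; The interaction interface drives custom-depth highlighting and the nearest-interaction widget on focus, and flips IsPressed on interact.
; A multicast event plays or reverses a timeline meant to lerp button height and light intensity.
; Sphere overlaps by the local player character show the prompt, or hide it and clear the highlight.
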(event OnComponentBeginOverlap(Sphere)
  (params (OverlappedComponent :type Primitive%20Component%20Object%20Reference) (OtherActor :type Actor%20Object%20Reference) (OtherComp :type Primitive%20Component%20Object%20Reference) (OtherBodyIndex :type Integer) (bFromSweep :type Boolean) (SweepResult :type Hit%20Result%20Structure%20%28by%20ref%29))
  ;[0.6445 0.8228 1 0.502] Local Overlap Event
  (if (== (Game|GetPlayerCharacter 0) OtherActor)
    (Utilities|Casting|CastToBP_InteractionCharacter OtherActor)
    (Development|SetHiddeninGame (Variables|Default|GetWidget) false false)))

(event OnComponentEndOverlap(Sphere)
  (params (OverlappedComponent :type Primitive%20Component%20Object%20Reference) (OtherActor :type Actor%20Object%20Reference) (OtherComp :type Primitive%20Component%20Object%20Reference) (OtherBodyIndex :type Integer))
  (bind _button (Variables|Default|GetButton))
  (bind _widget (Variables|Default|GetWidget))
  ;[0.6445 0.8228 1 0.502] Local Overlap Event
  (if (== OtherActor (Game|GetPlayerCharacter 0))
    (Utilities|Casting|CastToBP_InteractionCharacter OtherActor)
    (Rendering|SetRenderCustomDepth _button false)
    (Rendering|SetCustomDepthStencilValue _button 0)
    (if (Rendering|IsVisible _widget)
      (Development|SetHiddeninGame _widget true false))))

(event Custom|Pressed%20Button%20%28multicast%29
  (params (IsPressed? :type Boolean))
  ;[1 1 1 0.5] Pressed Button (multicast)
  (if IsPressed?
    (Audio|Components|Audio|Play (Variables|Default|GetTimeline%20Button))
    (else
      (Utilities|String|Reverse (Variables|Default|GetTimeline%20Button)))))

(event EventFocusInteraction
  (params (Focused :type Boolean))
  (bind _button (Variables|Default|GetButton))
  (bind _widget (Variables|Default|GetWidget))
  (bind _widget_2 (Variables|Default|GetWidget))
  (bind _button_2 (Variables|Default|GetButton))
  ;[1 1 1 0.5] Focus Interaction (interface)
  (if Focused
    ;[0.6445 0.8228 1 0.502] Local Visual
    (Rendering|SetRenderCustomDepth _button_2 true)
    (Rendering|SetCustomDepthStencilValue _button_2 2)
    (if (Rendering|IsVisible _widget_2)
      _
      (else
        (Development|SetHiddeninGame _widget_2 false false)))
    (Default|OnFocused (Variables|Default|GetAs%20WBP%20Nearest%20Interaction) true)
    (else
      (Rendering|SetRenderCustomDepth _button false)
      (Rendering|SetCustomDepthStencilValue _button 0)
      (if (Rendering|IsVisible _widget)
        _
        (else
          (Development|SetHiddeninGame _widget true false)))
      (Default|OnFocused (Variables|Default|GetAs%20WBP%20Nearest%20Interaction) false))))

(event EventBeginPlay
  ;[1 1 1 0.5] Begin Play
  (bind _aswbp_nearest_interaction (Utilities|Casting|CastToWBP_NearestInteraction (UserInterface|GetWidget (Variables|Default|GetWidget))))
  (Variables|Default|SetAs%20WBP%20Nearest%20Interaction _aswbp_nearest_interaction))

(event EventInteractwithActor
  ;[1 1 1 0.5] Interact With Actor (interface)
  (if (Variables|Default|GetIsPressed?)
    (Variables|Default|SetIsPressed? false)
    (else
      (Variables|Default|SetIsPressed? true)))
  (CallFunction|PressedButton(multicast) (Variables|Default|GetIsPressed?)))

(fn ConstructionScript)