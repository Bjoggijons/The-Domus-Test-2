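; BP_LightWithOverlap is a networked light actor whose spotlight fades on while a BP_InteractionCharacter is inside its box and fades off on exit.
; Box begin and end overlaps pass an on/off flag through a server event to a multicast event.
; The multicast plays or reverses a timeline whose alpha interpolates the spotlight intensity between zero and full.
; Exits are not counted, so any character leaving starts the fade-out.
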(event OnComponentBeginOverlap(Box)
  (params (OverlappedComponent :type Primitive%20Component%20Object%20Reference) (OtherActor :type Actor%20Object%20Reference) (OtherComp :type Primitive%20Component%20Object%20Reference) (OtherBodyIndex :type Integer) (bFromSweep :type Boolean) (SweepResult :type Hit%20Result%20Structure%20%28by%20ref%29))
  ;[1 1 1 0.5] Overlap Event
  (Utilities|Casting|CastToBP_InteractionCharacter OtherActor)
  (CallFunction|ActiveLight(server) true))

(event OnComponentEndOverlap(Box)
  (params (OverlappedComponent :type Primitive%20Component%20Object%20Reference) (OtherActor :type Actor%20Object%20Reference) (OtherComp :type Primitive%20Component%20Object%20Reference) (OtherBodyIndex :type Integer))
  ;[1 1 1 0.5] Overlap Event
  (Utilities|Casting|CastToBP_InteractionCharacter OtherActor)
  (CallFunction|ActiveLight(server) false))

(event Custom|Active%20Light%20%28server%29
  (params (IsActive? :type Boolean))
  ;[1 1 1 0.5] Active Light (server)
  (CallFunction|ActiveLight(multicast) IsActive?))

(event Custom|Active%20Light%20%28multicast%29
  (params (IsActive? :type Boolean))
  (bind _timeline_light (Variables|Default|GetTimeline%20Light))
  ;[1 1 1 0.5] Active Light (multicast)
  (if IsActive?
    (Audio|Components|Audio|Play _timeline_light)
    (else
      (Utilities|String|Reverse _timeline_light))))

(fn ConstructionScript)