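; Game mode for the interaction system that tracks connected player controllers and spawns their characters.
; Login, controller swap and logout events maintain the controller array, with login also storing the newest array index as PlayerIndex.
; An interface SpawnPlayer request destroys any existing pawn, then spawns and possesses a BP_InteractionCharacter.
; The spawn transform comes from the PlayerStart at that shared PlayerIndex, with no occupancy check.
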(event EventPostLogin
  (params (NewPlayer :type Player%20Controller%20Object%20Reference))
  ;[1 1 1 0.5] Connect Player
  (bind _returnvalue (Utilities|Array|Add (Variables|Default|GetNewPlayer) NewPlayer))
  (Variables|Default|SetPlayerIndex _returnvalue))

(event EventOnSwapPlayerControllers
  (params (OldPC :type Player%20Controller%20Object%20Reference) (NewPC :type Player%20Controller%20Object%20Reference))
  ;[1 1 1 0.5] Connect Player
  (Utilities|Array|Add (Variables|Default|GetNewPlayer) NewPC))

(event EventOnLogout
  (params (ExitingController :type Controller%20Object%20Reference))
  ;[1 1 1 0.5] Disconnect Player
  (bind _asplayer_controller (Utilities|Casting|CastToPlayerController ExitingController))
  (Utilities|Array|RemoveItem (Variables|Default|GetNewPlayer) _asplayer_controller))

(event EventSpawnPlayer
  (params (PC :type Player%20Controller%20Object%20Reference))
  ;[1 1 1 0.5] Request Spawn Player (interface)
  (CallFunction|SpawnPlayeratAvailableStartLocation PC))

(fn ConstructionScript)

(fn SpawnPlayeratAvailableStartLocation
  (params (PC :type Player%20Controller%20Object%20Reference))
  (bind _returnvalue (Pawn|GetControlledPawn PC))
  ;[1 1 1 0.5] Pawn exist?
  (Utilities|IsValid _returnvalue
    (:Is%20Valid
      (Actor|DestroyActor _returnvalue))
    (:Is%20Not%20Valid
      _))
  ;[1 1 1 0.5] Spawn (new) Pawn and Possess
  (bind _returnvalue_2 (Game|SpawnActorfromClass "/Game/InteractionSystem/Character/BP_InteractionCharacter.BP_InteractionCharacter_C" (CallFunction|GetPlayerStartLocation) "Undefined" "MultiplyWithRoot" 0 0))
  (Pawn|Possess PC _returnvalue_2))

(fn GetPlayerStartLocation
  (bind _outactors (Actor|GetAllActorsOfClass "/Script/Engine.PlayerStart"))
  (return (Transformation|GetActorTransform (Utilities|Array|Get(acopy) _outactors (Variables|Default|GetPlayerIndex)))))