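; Player controller for the interaction system that requests the player's spawn and sets up input on the local client.
; On BeginPlay, only the local controller calls a server RPC, which asks the game mode to spawn the player through a message call.
; It then adds the interaction Enhanced Input mapping context and switches to game-only input mode if the input subsystem is valid.
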(event Custom|Spawn%20Player%20%28server%29
  ;[1 1 1 0.5] Spawn Player (server)
  (Class|BPIGM|SpawnPlayer(Message) (Game|GetGameMode) self))

(event EventBeginPlay
  (bind _returnvalue (PlayerController|LocalPlayerSubsystems|GetEnhancedInputLocalPlayerSubsystem))
  (if (Pawn|IsLocalController)
    ;[1 1 1 0.5] Spawn Player (server)
    (CallFunction|SpawnPlayer(server))
    ;[1 1 1 0.5] Add Mapping Context
    (Utilities|IsValid _returnvalue
      (:Is%20Valid
        (Input|AddMappingContext _returnvalue "/Game/InteractionSystem/Character/Inputs/IMC_Interaction.IMC_Interaction" 0 "(bIgnoreAllPressedKeysUntilRelease=True,bForceImmediately=False,bNotifyUserSettings=False)")
        (Input|SetInputModeGameOnly self false)))))

(fn ConstructionScript)