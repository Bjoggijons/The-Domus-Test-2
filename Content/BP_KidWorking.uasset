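; BP_KidWorking is a pawn for a "Finish The Paper" task that hides itself when unpossessed.
; On BeginPlay it creates a UI_PopUp widget and sets that objective text on it.
; It then clears the LockCursor flag on the first-person character's crosshair, if that character is the player pawn, and enables click events and the mouse cursor on the player controller.
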(event Custom|UpdateText
  (Default|UpdateObjectiveText (Variables|Default|GetUI_Paper_Ref) "Finish The Paper"))

(event Custom|LockCursor
  (bind _asbp_first_person_character (Utilities|Casting|CastToBP_FirstPersonCharacter (Game|Player|GetPlayerPawn 0)))
  (Variables|/Game/Crosshair/UI_Crosshair.UI_Crosshair_C|SetLockCursor (Variables|/Game/FirstPerson/Blueprints/BP_FirstPersonCharacter.BP_FirstPersonCharacter_C|GetCrosshairRef _asbp_first_person_character) false))

(event Custom|clicking
  (bind _returnvalue (Game|GetPlayerController 0))
  (Variables|/Script/Engine.PlayerController|SetbEnableClickEvents _returnvalue true)
  (Variables|/Script/Engine.PlayerController|SetbShowMouseCursor _returnvalue true))

(event EventUnpossessed
  (params (OldController :type Controller%20Object%20Reference))
  (Rendering|SetActorHiddenInGame true))

(event EventBeginPlay
  (bind _returnvalue (UserInterface|CreateWidget "/Game/FirstPerson/UI_PopUp.UI_PopUp_C"))
  (Variables|Default|SetUI_Paper_Ref _returnvalue)
  (UserInterface|Viewport|AddtoViewport _returnvalue 0)
  (CallFunction|UpdateText)
  (CallFunction|LockCursor)
  (CallFunction|Clicking))

(fn ConstructionScript)