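; BP_Door_04 is a swinging door that toggles open and closed, with the motion multicast for multiplayer.
; The IsDoorOpen event flips the DoorIsOpen flag and passes it to a multicast event, which plays or reverses a Timeline.
; The Timeline's alpha interpolates the relative yaw of the SMDoor03 component to swing it between closed and open.
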(event Custom|Open%20Door%20%28multicast%29
  (params (DoorIsOpen? :type Boolean))
  (bind _timeline (Variables|Default|GetTimeline))
  ;[1 1 1 0.5] Open Door (multicast)
  (if DoorIsOpen?
    (Audio|Components|Audio|Play _timeline)
    (else
      (Utilities|String|Reverse _timeline))))

(event Custom|IsDoorOpen
  ;[0.15 0.15 0.15 0.5] IsDoorOpen
  (if (Variables|Default|GetDoorIsOpen?)
    (Variables|Default|SetDoorIsOpen? false)
    (else
      (Variables|Default|SetDoorIsOpen? true)))
  (CallFunction|OpenDoor(multicast) (Variables|Default|GetDoorIsOpen?)))

(fn ConstructionScript)