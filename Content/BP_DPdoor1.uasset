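; BP_DPdoor1 is a level-exit door that stays locked until the padlock puzzle is solved.
; On BeginPlay it caches the padlock and first-person player actors found in the level.
; When the box trigger is overlapped, it checks the padlock's Done flag; if set and the overlapper is the player, it opens FloorLevel1 and updates the objective popup to "Answer The Door".
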(event OnComponentBeginOverlap(Box)
  (params (OverlappedComponent :type Primitive%20Component%20Object%20Reference) (OtherActor :type Actor%20Object%20Reference) (OtherComp :type Primitive%20Component%20Object%20Reference) (OtherBodyIndex :type Integer) (bFromSweep :type Boolean) (SweepResult :type Hit%20Result%20Structure%20%28by%20ref%29))
  (bind _playerref (Variables|Default|GetPlayerRef))
  (bind _ui_popup (Variables|/Game/FirstPerson/Blueprints/BP_FirstPersonCharacter.BP_FirstPersonCharacter_C|GetUI_PopUp _playerref))
  (CallFunction|PuzzleDone)
  (if (Variables|Default|GetPadlockDone)
    (Utilities|Casting|CastToBP_FirstPersonCharacter OtherActor)
    (Game|OpenLevel(byObjectReference) "/Game/FloorLevel1.FloorLevel1")
    (Default|UpdateObjectiveText _ui_popup)
    (UserInterface|Viewport|AddtoViewport _ui_popup 0)
    (Default|UpdateObjectiveText _ui_popup "Answer The Door")
    (UserInterface|Viewport|AddtoViewport _ui_popup 0)))

(event Custom|PuzzleDone
  (if (Variables|/Game/BP_Padlock.BP_Padlock_C|GetDone (Variables|Default|GetPadlockRef))
    (Variables|Default|SetPadlockDone true)))

(event EventBeginPlay
  (bind _returnvalue (Actor|GetActorOfClass "/Game/BP_Padlock.BP_Padlock_C"))
  (Variables|Default|SetPadlockRef _returnvalue)
  (bind _returnvalue_2 (Actor|GetActorOfClass "/Game/FirstPerson/Blueprints/BP_FirstPersonCharacter.BP_FirstPersonCharacter_C"))
  (Variables|Default|SetPlayerRef _returnvalue_2))

(fn ConstructionScript)