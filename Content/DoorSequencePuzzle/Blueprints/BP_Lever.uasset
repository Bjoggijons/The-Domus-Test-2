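; BP_Lever is an interactable lever switch for the door sequence puzzle that toggles between off and on.
; An overlap box registers it as the demo character's current interacting item.
; Each interaction flip-flops a timeline that rotates the arm, setting the activated state and firing SwitchActivated or SwitchDeactivated when it finishes.
; CEDeactivate reuses the interaction to switch an activated lever back off, keeping the toggle in step.
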(event OnComponentBeginOverlap(Box)
  (params (OverlappedComponent :type Primitive%20Component%20Object%20Reference) (OtherActor :type Actor%20Object%20Reference) (OtherComp :type Primitive%20Component%20Object%20Reference) (OtherBodyIndex :type Integer) (bFromSweep :type Boolean) (SweepResult :type Hit%20Result%20Structure%20%28by%20ref%29))
  (bind _asbp_third_person_character_demo (Utilities|Casting|CastToBP_DemoCharacter OtherActor))
  (Variables|/Game/DoorSequencePuzzle/Characters/BP_DemoCharacter.BP_DemoCharacter_C|SetCurrentInteractingItem _asbp_third_person_character_demo self))

(event OnComponentEndOverlap(Box)
  (params (OverlappedComponent :type Primitive%20Component%20Object%20Reference) (OtherActor :type Actor%20Object%20Reference) (OtherComp :type Primitive%20Component%20Object%20Reference) (OtherBodyIndex :type Integer))
  (bind _asbp_third_person_character_demo (Utilities|Casting|CastToBP_DemoCharacter OtherActor))
  (Variables|/Game/DoorSequencePuzzle/Characters/BP_DemoCharacter.BP_DemoCharacter_C|SetCurrentInteractingItem _asbp_third_person_character_demo 0))

(event Custom|OnInteract
  (Utilities|FlowControl|FlipFlop
    (:A
      (bind (_direction _alpha) (Timeline|Timeline Play)
        (:Update
          (Transformation|SetRelativeRotation (Variables|Default|GetLeverArm) (Math|Rotator|Lerp(Rotator) (Variables|Default|GetLeverOffRotation) (Variables|Default|GetLeverOnRotation) _alpha) false false))
        (:Finished
          (switch Utilities|FlowControl|Switch|SwitchonETimelineDirection _direction
            (:Forward
              (Variables|Default|SetbIsActivated true)
              (Default|CallSwitchActivated self))
            (:Backward
              (Variables|Default|SetbIsActivated false)
              (Default|CallSwitchDeactivated self))))))
    (:B
      (Timeline|Timeline Reverse))))

(event EventBeginPlay
  (Transformation|SetRelativeRotation (Variables|Default|GetLeverArm) (Variables|Default|GetLeverOffRotation) false false))

(event EventCEDeactivate
  (if (Variables|Default|GetbIsActivated)
    (CallFunction|OnInteract)))

(fn ConstructionScript
  (|CallParentFunction))