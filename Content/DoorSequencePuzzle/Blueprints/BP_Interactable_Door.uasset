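; Interactable puzzle door that swings open and closed on a timeline-driven yaw rotation.
; At BeginPlay it picks one of three modes: driven by a DirectSolver switch, by its sequence puzzle component's activators, or automatic when neither is set.
; Sequence solved and unsolved events act only when their owner is this door.
; In automatic mode, a BP_DemoCharacter hit opens the door, then closes it after a delay.
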(event OnComponentHit(Door)
  (params (HitComponent :type Primitive%20Component%20Object%20Reference) (OtherActor :type Actor%20Object%20Reference) (OtherComp :type Primitive%20Component%20Object%20Reference) (NormalImpulse :type Vector :default "0, 0, 0") (Hit :type Hit%20Result%20Structure%20%28by%20ref%29))
  ;[0.15 0.15 0.15 0.5] Automatic Door openning closing handle by player hit
  (Utilities|FlowControl|Sequence
    (:then_0
      (if (Variables|Default|GetbIsAutomatic)
        (Utilities|Casting|CastToBP_DemoCharacter OtherActor)
        (CallFunction|CEonOpen)
        (Utilities|FlowControl|Delay 5.0)
        (CallFunction|CEonClose)))))

(event Custom|CE_OnClose
  (if (Variables|Default|GetisOpen)
    (Variables|Default|SetisOpen false)
    (bind _rotation (Timeline|DoorOpen Reverse)
      (:Update
        (Transformation|SetRelativeRotation (Variables|Default|GetDoor) (Math|Rotator|MakeRotator 0.0 0.0 _rotation) false false)))))

(event Custom|CE_OnOpen
  (if (not (Variables|Default|GetisOpen))
    (Variables|Default|SetisOpen true)
    (bind _rotation (Timeline|DoorOpen Play)
      (:Update
        (Transformation|SetRelativeRotation (Variables|Default|GetDoor) (Math|Rotator|MakeRotator 0.0 0.0 _rotation) false false)))))

(event Custom|CE_PuzzleSolved
  (params (Solver :type BP%20Puzzle%20Sover%20Object%20Reference))
  ;[0.15 0.15 0.15 0.5] Handle Door Interaction without Puzzle
  (CallFunction|CEonOpen))

(event Custom|CE_PuzzleUnsolved
  (params (Solver :type BP%20Puzzle%20Sover%20Object%20Reference))
  ;[0.15 0.15 0.15 0.5] Handle Door Interaction without Puzzle
  (CallFunction|CEonClose))

(event Custom|CE_SequencePuzzleUnsolved
  (params (DeactivateOwner :type Actor%20Object%20Reference))
  ;[0.15 0.15 0.15 0.5] Handle when Door can be open after valid Sequence Triggered with Solver
  (if (== DeactivateOwner self)
    (CallFunction|CEonClose)))

(event Custom|CE_SequencePuzzleSolved
  (params (ActivateOwner :type Actor%20Object%20Reference))
  ;[0.15 0.15 0.15 0.5] Handle when Door can be open after valid Sequence Triggered with Solver
  (if (== ActivateOwner self)
    (CallFunction|CEonOpen)))

(event EventBeginPlay
  (Utilities|IsValid (Variables|Default|GetDirectSolver)
    (:Is%20Valid
      ;[0.15 0.15 0.15 0.5] Handle Door Interaction without Puzzle
      (EventDispatchers|BindEventtoSwitchActivated (Variables|Default|GetDirectSolver) (delegate Custom|CE_PuzzleSolved))
      (EventDispatchers|BindEventtoSwitchDeactivated (Variables|Default|GetDirectSolver) (delegate Custom|CE_PuzzleUnsolved)))
    (:Is%20Not%20Valid
      (Utilities|Array|RemoveItem (Variables|/Game/DoorSequencePuzzle/Components/BP_SequencePuzzleComponent.BP_SequencePuzzleComponent_C|GetPuzzleActivators (Variables|Default|GetBP_SequencePuzzleComponent)) 0)
      ;[0.15 0.15 0.15 0.5] Handle when Door can be open after valid Sequence Triggered with Solver
      (if (Utilities|Array|IsNotEmpty (Variables|/Game/DoorSequencePuzzle/Components/BP_SequencePuzzleComponent.BP_SequencePuzzleComponent_C|GetPuzzleActivators (Variables|Default|GetBP_SequencePuzzleComponent)))
        (Default|CEEnablePuzzle (Variables|Default|GetBP_SequencePuzzleComponent))
        (EventDispatchers|BindEventtoPuzzleSolved (Variables|Default|GetBP_SequencePuzzleComponent) (delegate Custom|CE_SequencePuzzleSolved))
        (EventDispatchers|BindEventtoPuzzleUnsolved (Variables|Default|GetBP_SequencePuzzleComponent) (delegate Custom|CE_SequencePuzzleUnsolved))
        (else
          ;[0.15 0.15 0.15 0.5] Handle when Door is open without any Solver (automatic door)
          (Variables|Default|SetbIsAutomatic true))))))

(fn ConstructionScript)