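; Puzzle component that validates the activation order of linked switch actors and dispatches solved or unsolved events with its owner, such as a door.
; It binds to each activator's events, tracking progress under three modes: Sequential Strict resets all on error, Sequential Lenient rejects only the wrong switch, Unordered needs all active.
; Undoing an earlier sequential step cascades deactivation to later ones, guarded against re-entry.
; Debug widgets display switch names and the expected order.
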(event Custom|CE_EnablePuzzle
  ;[0.15 0.15 0.15 0.5] Enable Puzzle System :
  ; 1. Display Puzzle lever sequence at top of solver/switch and door
  ; 2. Receive Switch/Solver activation or Deactivation dispatched event)
  (for _array_element (Variables|Default|GetPuzzleActivators)
    (EventDispatchers|AssignSwitchActivated _array_element (EventDispatchers|CreateEvent :!event Custom|CE_SwitchActivated))
    (EventDispatchers|AssignSwitchDeactivated _array_element (EventDispatchers|CreateEvent :!event Custom|CE_SwitchDeactivated))
    (CallFunction|FShowSolverName _array_element))
  (CallFunction|FShowPuzzleSequence)
  (CallFunction|FUpdatePuzzleSequence))

(event Custom|CE_SwitchActivated
  (params (Solver :type BP%20Puzzle%20Sover%20Object%20Reference))
  ;[0.15 0.15 0.15 0.5] 1. Handle Solver/Switch activation
  ; 2. Verify Puzzle solved in sequence otherwise deactivate Solver/switch based on Puzzle Verification Mode
  (if (not (Variables|Default|GetbIsSolved))
    (switch Utilities|FlowControl|Switch|SwitchonE_DoorPuzzleValidationMode (Variables|Default|GetValidationMode)
      (:NewEnumerator1
        (if (== Solver (Utilities|Array|Get(acopy) (Variables|Default|GetPuzzleActivators) (Variables|Default|GetCurrentStep))) :!label _label
          (CallFunction|FValidActivation)
          (else
            (CallFunction|FInvalidActivation Solver))))
      (:NewEnumerator0
        (goto _label))
      (:NewEnumerator2
        (CallFunction|CECheckUnorderedWinCondition)))))

(event Custom|CE_SwitchDeactivated
  (params (Solver :type BP%20Puzzle%20Sover%20Object%20Reference))
  (bind _puzzleactivators (Variables|Default|GetPuzzleActivators))
  (bind _returnvalue (Utilities|Array|FindItem _puzzleactivators Solver))
  ;[0.15 0.15 0.15 0.5] 1. Handle Solver/Switch Deactivation Event
  ; 2. Deactivate if  Solver/switches after the selected Solver/Switch
  ; 3. Mark Puzzle Unsolved
  (if (not (Variables|Default|GetbIsInternallyDeactivating))
    (switch Utilities|FlowControl|Switch|SwitchonE_DoorPuzzleValidationMode (Variables|Default|GetValidationMode)
      (:NewEnumerator1
        (if (< _returnvalue (Variables|Default|GetCurrentStep)) :!label _label
          (CallFunction|FSequenceSwitchDeactivation _returnvalue (Variables|Default|GetCurrentStep))))
      (:NewEnumerator0
        (goto _label))
      (:NewEnumerator2
        (CallFunction|CEPuzzleUnsolved)))))

(event Custom|CE_PuzzleUnsolved
  ;[0.15 0.15 0.15 0.5] Mark Puzzle Unsolved and Dispatch Event that puzzle is unsolved
  (Variables|Default|SetbIsSolved false)
  (Default|CallPuzzleUnsolved (Components|GetOwner)))

(event Custom|CE_PuzzleSolved
  ;[0.15 0.15 0.15 0.5] Mark Puzzle Solveed and Dispatch Event that Puzzle is solved
  (Variables|Default|SetbIsSolved true)
  (Default|CallPuzzleSolved (Components|GetOwner)))

(event Custom|CE_CheckUnorderedWinCondition
  (bind _puzzleactivators (Variables|Default|GetPuzzleActivators))
  ;[0.15 0.15 0.15 0.5] Unorder Puzzle Varication Win condtion Handling
  (bind _array_element (Utilities|Array|ForEachLoopwithBreak _puzzleactivators :!label _label)
    (:LoopBody
      (if (Variables|/Game/DoorSequencePuzzle/Blueprints/BP_PuzzleSover.BP_PuzzleSover_C|GetbIsActivated _array_element)
        (Math|Integer|IncrementInt (Variables|Default|GetCurrentStep))
        (else
          (goto _label Break))))
    (:Completed
      (if (== (Variables|Default|GetCurrentStep) (Utilities|Array|Length _puzzleactivators))
        (CallFunction|CEPuzzleSolved)
        (Variables|Default|SetCurrentStep 0)
        (else
          (Variables|Default|SetCurrentStep 0))))))

(fn FIsForceDeactivationAllowed
  (params (Solver :type BP%20Puzzle%20Sover%20Object%20Reference))
  ;[0.15 0.15 0.15 0.5] Validate that selected solver can mark Deactivated forcefully like auto off if incorrect sequence triggered
  (if true
    (return true)
    (else
      (return false))))

(fn FValidActivation
  (bind _currentstep (Variables|Default|GetCurrentStep))
  (bind _puzzleactivators (Variables|Default|GetPuzzleActivators))
  (bind _output (Utilities|Array|Get(acopy) _puzzleactivators _currentstep))
  ;[0.15 0.15 0.15 0.5] Perform puzzle solve validation after Valid move in puzzle sequence
  (Math|Integer|IncrementInt (Variables|Default|GetCurrentStep)
    (:%20%20
      (if (< (Variables|Default|GetCurrentStep) (Utilities|Array|Length (Variables|Default|GetPuzzleActivators))) :!label _label
        (if (and (CallFunction|FIsForceDeactivationAllowed _output) (Variables|/Game/DoorSequencePuzzle/Blueprints/BP_PuzzleSover.BP_PuzzleSover_C|GetbIsActivated _output))
          (Math|Integer|IncrementInt (Variables|Default|GetCurrentStep)
            (:%20%20
              (goto _label)))
          (elif (== (Variables|Default|GetCurrentStep) (Utilities|Array|Length (Variables|Default|GetPuzzleActivators)))
            (CallFunction|CEPuzzleSolved)))
        (else
          (CallFunction|CEPuzzleSolved))))))

(fn FInvalidActivation
  (params (InvalidSolver :type BP%20Puzzle%20Sover%20Object%20Reference))
  ;[0.15 0.15 0.15 0.5] Perform next solver Deactivation based on Verification Mode
  ; 1. Sequential Strict - All Solvers Deactivated, player needs to start from the beginning
  ; 2. Sequential Lenient - only invalid Solver Deactivated, player needs to find the valid sequence
  ; 3. Unordered - nothing on invalid activation because no sequence matters​
  (switch Utilities|FlowControl|Switch|SwitchonE_DoorPuzzleValidationMode (Variables|Default|GetValidationMode)
    (:NewEnumerator1
      (for _array_element (Variables|Default|GetPuzzleActivators)
        (Default|CEDeactivate _array_element))
      (Variables|Default|SetCurrentStep 0)
      (CallFunction|CEPuzzleUnsolved))
    (:NewEnumerator0
      (Default|CEDeactivate InvalidSolver))))

(fn FSequenceSwitchDeactivation
  (params (SolverIndex :type Integer) (OldCurrentStep :type Integer))
  ;[0.15 0.15 0.15 0.5] Perform an action if the solver is deactivated by an invalid move or the player disables it.
  ; 1. deactivate selected solver
  ; 2. deactivate upcoming active solver based on puzzle sequence
  (Variables|Default|SetCurrentStep SolverIndex)
  (Variables|Default|SetbIsInternallyDeactivating true)
  (for _index (range (+ SolverIndex 1) (- OldCurrentStep 1))
    (Default|CEDeactivate (Utilities|Array|Get(acopy) (Variables|Default|GetPuzzleActivators) _index)))
  (Variables|Default|SetbIsInternallyDeactivating false)
  (if (Variables|Default|GetbIsSolved)
    (CallFunction|CEPuzzleUnsolved)))

(fn FShowPuzzleSequence
  ;[0.15 0.15 0.15 0.5] Display Solver Sequnce above door (for debug purpose)
  (bind _returnvalue (UserInterface|CreateWidget "/Game/DoorSequencePuzzle/UI/WBP_InteractionPrompt.WBP_InteractionPrompt_C"))
  (bind _structout (Utilities|Struct|SetmembersinSlateFontInfo (Variables|/Script/UMG.TextBlock|GetFont (Variables|/Game/DoorSequencePuzzle/UI/WBP_InteractionPrompt.WBP_InteractionPrompt_C|GetInteractionTextBlock _returnvalue)) 1e+01))
  (Class|TextBlock|SetFont (Variables|/Game/DoorSequencePuzzle/UI/WBP_InteractionPrompt.WBP_InteractionPrompt_C|GetInteractionTextBlock _returnvalue) _structout)
  (bind _returnvalue_2 (Game|AddComponentbyClass (Components|GetOwner) "/Script/UMG.WidgetComponent" false (Math|Transform|MakeTransform "20.000000,-90.000000,300.000000" "0, 0, 0" "1.000000,1.000000,1.000000")))
  (UserInterface|SetWidget _returnvalue_2 _returnvalue))

(fn FShowSolverName
  (params (Target :type BP%20Puzzle%20Sover%20Object%20Reference))
  ;[0.15 0.15 0.15 0.5] Display solver name (for debug purpose)
  (bind _returnvalue (UserInterface|CreateWidget "/Game/DoorSequencePuzzle/UI/WBP_InteractionPrompt.WBP_InteractionPrompt_C"))
  (bind _structout (Utilities|Struct|SetmembersinSlateFontInfo (Variables|/Script/UMG.TextBlock|GetFont (Variables|/Game/DoorSequencePuzzle/UI/WBP_InteractionPrompt.WBP_InteractionPrompt_C|GetInteractionTextBlock _returnvalue)) 1e+01))
  (Class|TextBlock|SetFont (Variables|/Game/DoorSequencePuzzle/UI/WBP_InteractionPrompt.WBP_InteractionPrompt_C|GetInteractionTextBlock _returnvalue) _structout)
  (Variables|/Game/DoorSequencePuzzle/UI/WBP_InteractionPrompt.WBP_InteractionPrompt_C|SetTextPrompt _returnvalue (Utilities|Text|ToText(String) (Utilities|GetDisplayName Target)))
  (bind _returnvalue_2 (Game|AddComponentbyClass Target "/Script/UMG.WidgetComponent" false (Math|Transform|MakeTransform "125.000000,50.000000,200.000000" "0.000000,90.000000,0.000000" "1.000000,1.000000,1.000000")))
  (UserInterface|SetWidget _returnvalue_2 _returnvalue))

(fn FUpdatePuzzleSequence
  ;[0.15 0.15 0.15 0.5] Create and set puzzle sequence above door (for debug puspose)
  (LocalVariables|SetPuzzleOrder "")
  (for _array_element (Variables|Default|GetPuzzleActivators)
    (LocalVariables|SetPuzzleOrder (Utilities|String|Append (LocalVariables|GetPuzzleOrder) (Utilities|GetDisplayName _array_element) "
")))
  (bind _aswbp_interaction_prompt (Utilities|Casting|CastToWBP_InteractionPrompt (UserInterface|GetWidget (Actor|GetComponentbyClass (Components|GetOwner) "/Script/UMG.WidgetComponent"))))
  (Variables|/Game/DoorSequencePuzzle/UI/WBP_InteractionPrompt.WBP_InteractionPrompt_C|SetTextPrompt _aswbp_interaction_prompt (Utilities|Text|ToText(String) (LocalVariables|GetPuzzleOrder))))