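; AI enemy pawn with wander, search, chase and attack behaviors against the first-person player, still in prototype form.
; Looping timers drive wandering and attack-range checks from boolean state flags, with movement through AIMoveTo.
; Perception stimuli within detection range lead to a chase, with debug prints.
; Line-of-sight logic is disconnected, so CanSeePlayer is never set, and the attack only stops movement and sets flags, without damage.
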(event OnPerceptionUpdated(AIPerception)
  (params (UpdatedActors :type Array%20of%20Actor%20Object%20References))
  ;[0.15 0.15 0.15 0.5] Ckecking for player
)

(event OnTargetPerceptionUpdated(AIPerception)
  (params (Actor :type Actor%20Object%20Reference) (Stimulus :type AI%20Stimulus%20Structure))
  (if (<= (Math|Vector|Distance(Vector) (.stimuluslocation Stimulus) (Transformation|GetActorLocation self)) (Variables|Default|GetDetectionRange))
    (AI|AIMoveTo self "0, 0, 0" 0 5.0 false
      (:then
        (Variables|Default|SetHeardNoise true)
        (if (Variables|Default|GetHeardNoise)
          (if true
            (CallFunction|ChasePlayer)
            (Development|PrintString "working")
            (else
              (Development|PrintString "Distance failing"))))))))

(event Custom|SearchForPlayer
  ;[0.15 0.15 0.15 0.5] SearchForPlayer
  (if (Variables|Default|GetbIsSearching)
    (AI|AIMoveTo 0 (Variables|Default|GetLastKnownPlayerLocation) 0 5e+01 false
      (:then
        (Transformation|SetActorRotation self)
        (Utilities|FlowControl|Delay (Variables|Default|GetSearchDuration%20))
        (if (Variables|Default|GetbCanSeePlayer)
          (Variables|Default|SetbIsSearching false)
          (else
            (Variables|Default|SetbIsSearching true)
            (Variables|Default|SetbIsWandering true)))))))

(event Custom|ChasePlayer
  ;[0.15 0.15 0.15 0.5] ChasePlayer
  (AI|AIMoveTo self "0, 0, 0" (Variables|Default|GetPlayerRef) 5.0 false))

(event Custom|AttempAttack
  ;[0.15 0.15 0.15 0.5] AttemptAttack
  (if (not (Variables|Default|GetbHasAttacked))
    (Variables|Default|SetbHasAttacked true)
    (AI|Navigation|StopMovement (Pawn|GetController))
    (CallFunction|ResetAttackCooldown)))

(event Custom|ResetAttackCooldown
  ;[0.15 0.15 0.15 0.5] ResetAttackCooldown
  (Variables|Default|SetbCanAttack true))

(event Custom|GoToRandomLocation
  ;[0.15 0.15 0.15 0.5] GoToRandomLocation
  (AI|AIMoveTo self (.RandomLocation (AI|Navigation|GetRandomReachablePointinRadius (Transformation|GetActorLocation) (Variables|Default|GetWanderRadius) 0 0)) 0 5.0 false
    (:then
      (Utilities|FlowControl|Delay (Variables|Default|GetWanderDelay))
      (CallFunction|GotoRandomLocation))))

(event EventBeginPlay
  ;[0.15 0.15 0.15 0.5] Walk
  (Variables|/Script/Engine.CharacterMovementComponent|SetMaxWalkSpeed (Variables|Character|GetCharacterMovement) (Variables|Default|GetSpeed))
  (bind _asbp_first_person_character (Utilities|Casting|CastToBP_FirstPersonCharacter (Game|GetPlayerCharacter 0)))
  (Variables|Default|SetPlayerRef _asbp_first_person_character)
  (Utilities|Time|SetTimerbyFunctionName 0 "ChaseTick_F" 0.2 true)
  (Utilities|Time|SetTimerbyFunctionName 0 "WanderTick_F" (Variables|Default|GetWanderDelay) true))

(fn ConstructionScript)

(fn WanderTickF
  ;[0.15 0.15 0.15 0.5] WanderTick
  (if (Variables|Default|GetbIsWandering)
    (CallFunction|GotoRandomLocation)))

(fn ChaseTickF
  (bind _returnvalue (Pawn|GetController))
  ;[0.15 0.15 0.15 0.5] ChaseTick
  (Utilities|IsValid (Variables|Default|GetPlayerRef)
    (:Is%20Valid
      (if (Variables|Default|GetbCanSeePlayer)
        (if (< (Transformation|GetDistanceTo (Variables|Default|GetPlayerRef)) (Variables|Default|GetAttack%20Range%20))
          (AI|Navigation|StopMovement _returnvalue)
          (CallFunction|AttempAttack))
        (elif (Variables|Default|GetbIsSearching)
          (AI|Navigation|StopMovement _returnvalue))))))