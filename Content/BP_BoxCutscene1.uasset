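; BP_BoxCutscene1 is a trigger box that plays the Cutscene1 level sequence and moves the game to the Basement level.
; When BP_FirstPersonCharacter overlaps the Box, it creates and plays a sequence player, then opens Basement after a fixed delay rather than on a finished event.
; It finds BP_KidWorking at BeginPlay and clears its IsInLevel1 flag after the level-open call.
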(event OnComponentBeginOverlap(Box)
  (params (OverlappedComponent :type Primitive%20Component%20Object%20Reference) (OtherActor :type Actor%20Object%20Reference) (OtherComp :type Primitive%20Component%20Object%20Reference) (OtherBodyIndex :type Integer) (bFromSweep :type Boolean) (SweepResult :type Hit%20Result%20Structure%20%28by%20ref%29))
  (Utilities|Casting|CastToBP_FirstPersonCharacter OtherActor)
  (bind _returnvalue (Sequencer|Player|CreateLevelSequencePlayer (Variables|Default|GetCutscene1)))
  (Sequencer|Player|Play _returnvalue :!class /Script/MovieScene.MovieSceneSequencePlayer)
  (Utilities|FlowControl|Delay 6.5)
  (Game|OpenLevel(byName) "Basement")
  (Variables|/Game/BP_KidWorking.BP_KidWorking_C|SetIsInLevel1 (Variables|Default|GetKidRef) false))

(event EventBeginPlay
  (bind _returnvalue (Actor|GetActorOfClass "/Game/BP_KidWorking.BP_KidWorking_C"))
  (Variables|Default|SetKidRef _returnvalue))

(fn ConstructionScript)