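; BP_Padlock is a clickable combination padlock that the player sets through an on-screen widget.
; Clicking it removes the first-person character's crosshair, opens WBP_PadlockUI with a reference back to the padlock, and switches to UI-only input with a cursor.
; UpdateCombination writes a digit into the current combination, then CheckCombination compares it to the correct one.
; The result only sets AllCorrect and prints debug text per match, with no unlock action here.
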(event OnClicked(combination_padlock)
  (params (TouchedComponent :type Primitive%20Component%20Object%20Reference) (ButtonPressed :type Key%20Structure :default "None"))
  (bind _returnvalue (Game|GetPlayerController 0))
  ;[0.15 0.15 0.15 0.5] OnClicked
  (bind _asbp_first_person_character (Utilities|Casting|CastToBP_FirstPersonCharacter (Game|GetPlayerCharacter 0)))
  (Variables|/Game/Crosshair/UI_Crosshair.UI_Crosshair_C|SetLockCursor (Variables|/Game/FirstPerson/Blueprints/BP_FirstPersonCharacter.BP_FirstPersonCharacter_C|GetCrosshairRef _asbp_first_person_character) false)
  (Widget|RemovefromParent (Variables|/Game/FirstPerson/Blueprints/BP_FirstPersonCharacter.BP_FirstPersonCharacter_C|GetCrosshairRef _asbp_first_person_character))
  (bind _returnvalue_2 (UserInterface|CreateWidget "/Game/WBP_PadlockUI.WBP_PadlockUI_C" 0 0))
  (bind _output_get (Variables|Default|SetLockWidgetRef _returnvalue_2))
  (Variables|/Game/WBP_PadlockUI.WBP_PadlockUI_C|SetPadlockRef _output_get self)
  (UserInterface|Viewport|AddtoViewport _returnvalue_2 0)
  (Input|SetInputModeUIOnly _returnvalue _returnvalue_2 "DoNotLock" false)
  (Variables|/Script/Engine.PlayerController|SetbShowMouseCursor _returnvalue true))

(event Custom|UpdateCombination
  (params (NumberIndex :type Integer) (Value :type Integer))
  ;[0.15 0.15 0.15 0.5] UpdateCombination
  (Utilities|Array|SetArrayElem (Variables|Default|GetCurrentCombination) NumberIndex Value true)
  (CallFunction|CheckCombination))

(event Custom|CheckCombination
  ;[0.15 0.15 0.15 0.5] CheckCombination
  (Variables|Default|SetAllCorrect true)
  (for _index (range 0 (- (Utilities|Array|Length (Variables|Default|GetCurrentCombination)) 1))
    (if (== (Utilities|Array|Get(acopy) (Variables|Default|GetCorrectCombination) _index) (Utilities|Array|Get(acopy) (Variables|Default|GetCurrentCombination) _index))
      (Development|PrintString "one correct")
      (else
        (Variables|Default|SetAllCorrect false)))))

(fn ConstructionScript)