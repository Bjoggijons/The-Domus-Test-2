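; Puzzle button actor that toggles a linked light between green and red when interacted with.
; BeginPlay finds the first BP_Light1 in the level; each Interact flip-flops that light's Cylinder and Sphere materials and updates IsOn.
; The button's Sphere drops briefly and returns after a delay, with HasBeenPushed blocking overlapping press motions but not the toggle itself.
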(event EventInteract
  (bind _lightref1 (Variables|Default|GetLightRef1))
  (bind _lightref1_2 (Variables|Default|GetLightRef1))
  (Utilities|FlowControl|FlipFlop
    (:A
      (Rendering|Material|SetMaterial (Variables|/Game/Button_Puzzle/BP_Light1.BP_Light1_C|GetCylinder _lightref1) 0 "/Game/Button_Puzzle/Color_Green.Color_Green")
      (Rendering|Material|SetMaterial (Variables|/Game/Button_Puzzle/BP_Light1.BP_Light1_C|GetSphere _lightref1) 0 "/Game/Button_Puzzle/Color_Green.Color_Green")
      (Variables|Default|SetIsOn true)
      (if (not (Variables|Default|GetHasBeenPushed))
        (Transformation|AddWorldOffset (Variables|Default|GetSphere) "0.000000,0.000000,-5.000000" false false)
        (Variables|Default|SetHasBeenPushed true)
        (Utilities|FlowControl|Delay 1.0)
        (Transformation|AddWorldOffset (Variables|Default|GetSphere) "0.000000,0.000000,5.000000" false false)
        (Variables|Default|SetHasBeenPushed false)))
    (:B
      (Rendering|Material|SetMaterial (Variables|/Game/Button_Puzzle/BP_Light1.BP_Light1_C|GetCylinder _lightref1_2) 0 "/Game/Button_Puzzle/Color_Red.Color_Red")
      (Rendering|Material|SetMaterial (Variables|/Game/Button_Puzzle/BP_Light1.BP_Light1_C|GetSphere _lightref1_2) 0 "/Game/Button_Puzzle/Color_Red.Color_Red")
      (Variables|Default|SetIsOn false)
      (if (not (Variables|Default|GetHasBeenPushed))
        (Transformation|AddWorldOffset (Variables|Default|GetSphere) "0.000000,0.000000,-5.000000" false false)
        (Variables|Default|SetHasBeenPushed true)
        (Utilities|FlowControl|Delay 1.0)
        (Transformation|AddWorldOffset (Variables|Default|GetSphere) "0.000000,0.000000,5.000000" false false)
        (Variables|Default|SetHasBeenPushed false)))))

(event EventBeginPlay
  (bind _returnvalue (Actor|GetActorOfClass "/Game/Button_Puzzle/BP_Light1.BP_Light1_C"))
  (Variables|Default|SetLightRef1 _returnvalue))

(fn ConstructionScript)