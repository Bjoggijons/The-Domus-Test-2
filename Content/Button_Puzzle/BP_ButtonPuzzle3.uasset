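; Third button of a button puzzle, which toggles its matching light between green and red when interacted with.
; On BeginPlay it finds and stores references to five light actors by class, though only the Light3 reference is used.
; Interact drives a FlipFlop that swaps the materials on that light's cylinder and sphere and records the state in IsOn0.
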(event EventInteract
  (bind _lightref3_0 (Variables|Default|GetLightRef3_0))
  (bind _lightref3_0_2 (Variables|Default|GetLightRef3_0))
  (Utilities|FlowControl|FlipFlop
    (:A
      (Rendering|Material|SetMaterial (Variables|/Game/Button_Puzzle/BP_Light3.BP_Light3_C|GetCylinder _lightref3_0) 0 "/Game/Button_Puzzle/Color_Green.Color_Green")
      (Rendering|Material|SetMaterial (Variables|/Game/Button_Puzzle/BP_Light3.BP_Light3_C|GetSphere _lightref3_0) 0 "/Game/Button_Puzzle/Color_Green.Color_Green")
      (Variables|Default|SetIsOn_0 true))
    (:B
      (Rendering|Material|SetMaterial (Variables|/Game/Button_Puzzle/BP_Light3.BP_Light3_C|GetCylinder _lightref3_0_2) 0 "/Game/Button_Puzzle/Color_Red.Color_Red")
      (Rendering|Material|SetMaterial (Variables|/Game/Button_Puzzle/BP_Light3.BP_Light3_C|GetSphere _lightref3_0_2) 0 "/Game/Button_Puzzle/Color_Red.Color_Red")
      (Variables|Default|SetIsOn_0 false))))

(event EventBeginPlay
  (bind _returnvalue (Actor|GetActorOfClass "/Game/Button_Puzzle/BP_Light1.BP_Light1_C"))
  (Variables|Default|SetLightRef1_0 _returnvalue)
  (bind _returnvalue_2 (Actor|GetActorOfClass "/Game/Button_Puzzle/BP_Light2.BP_Light2_C"))
  (Variables|Default|SetLightRef2_0 _returnvalue_2)
  (bind _returnvalue_3 (Actor|GetActorOfClass "/Game/Button_Puzzle/BP_Light3.BP_Light3_C"))
  (Variables|Default|SetLightRef3_0 _returnvalue_3)
  (bind _returnvalue_4 (Actor|GetActorOfClass "/Game/Button_Puzzle/BP_Light4.BP_Light4_C"))
  (Variables|Default|SetLightRef4_0 _returnvalue_4)
  (bind _returnvalue_5 (Actor|GetActorOfClass "/Game/Button_Puzzle/BP_Light5.BP_Light5_C"))
  (Variables|Default|SetLightRef5_0 _returnvalue_5))

(fn ConstructionScript)