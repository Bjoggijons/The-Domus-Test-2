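; BP_MainDoor is a main door that opens only when the player holds all four key flags, then leads to the final level.
; HasKeys checks the flags on the first-person character, then a timeline swings DoorA open in yaw, marks the door interacted and removes its UI prompt.
; A separate overlap event opens FinalLevel when the player enters.
; BeginPlay caches the player and two key actors, though the key references go unused here.
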(event OnComponentBeginOverlap()
  (params (OverlappedComponent :type Primitive%20Component%20Object%20Reference) (OtherActor :type Actor%20Object%20Reference) (OtherComp :type Primitive%20Component%20Object%20Reference) (OtherBodyIndex :type Integer) (bFromSweep :type Boolean) (SweepResult :type Hit%20Result%20Structure%20%28by%20ref%29))
  ;[0.15 0.15 0.15 0.5] HasKeys
  (Utilities|Casting|CastToBP_FirstPersonCharacter OtherActor)
  (Game|OpenLevel(byObjectReference) "/Game/FinalLevel.FinalLevel"))

(event Custom|HasKeys
  (bind _playerref (Variables|Default|GetPlayerRef))
  (bind _playerref_2 (Variables|Default|GetPlayerRef))
  ;[0.15 0.15 0.15 0.5] HasKeys
  (if (Math|Boolean|ANDBoolean (Variables|/Game/FirstPerson/Blueprints/BP_FirstPersonCharacter.BP_FirstPersonCharacter_C|GetHasFirstKey _playerref) (Variables|/Game/FirstPerson/Blueprints/BP_FirstPersonCharacter.BP_FirstPersonCharacter_C|GetHasSecondKey _playerref) (Variables|/Game/FirstPerson/Blueprints/BP_FirstPersonCharacter.BP_FirstPersonCharacter_C|GetHasFirstKey2 _playerref) (Variables|/Game/FirstPerson/Blueprints/BP_FirstPersonCharacter.BP_FirstPersonCharacter_C|GetHasSecondKey2 _playerref))
    (bind _alpha (Timeline|Timeline Play)
      (:Update
        (Transformation|SetRelativeRotation (Variables|Default|GetDoor_a) (Math|Rotator|MakeRotator 0.0 0.0 (Math|Float|Lerp 0.0 -1.2e+02 _alpha)) false false)
        (Variables|/Game/FirstPerson/Blueprints/BP_FirstPersonCharacter.BP_FirstPersonCharacter_C|SetHasInteractedMainDoor _playerref_2 true)
        (Widget|RemovefromParent (Variables|/Game/FirstPerson/Blueprints/BP_FirstPersonCharacter.BP_FirstPersonCharacter_C|GetUI_PromptMainDoor _playerref_2))))))

(event EventBeginPlay
  (bind _returnvalue (Actor|GetActorOfClass "/Game/Keys/BP_FirstFloorKey.BP_FirstFloorKey_C"))
  (Variables|Default|SetFirstFloorKey _returnvalue)
  (bind _returnvalue_2 (Actor|GetActorOfClass "/Game/Keys/BP_SecondFloorKey.BP_SecondFloorKey_C"))
  (Variables|Default|SetSecondFloorKey _returnvalue_2)
  (bind _returnvalue_3 (Actor|GetActorOfClass "/Game/FirstPerson/Blueprints/BP_FirstPersonCharacter.BP_FirstPersonCharacter_C"))
  (Variables|Default|SetPlayerRef _returnvalue_3))

(fn ConstructionScript)